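; Behavior tree task that cycles a stranger NPC through its list of target locations.
; On execute it advances the TargetListIndex blackboard key, wrapping to zero past the end of the pawn's TargetLocationList.
; It then writes that target actor's location to the CurrentTarget vector key and finishes successfully, leaving movement itself to other nodes.
; A pawn that is not a StrangerCharacter_BTVer stops execution without finishing the task.
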(event EventReceiveExecuteAI
  (params (OwnerController :type AI%20Controller%20Object%20Reference) (ControlledPawn :type Pawn%20Object%20Reference))
  (bind _targetlistindex (Variables|Default|GetTargetListIndex))
  (bind _returnvalue (Class|BTFunctionLibrary|GetBlackboardValueasInt _targetlistindex))
  (bind _returnvalue_2 (+ _returnvalue 1))
  (bind _asstranger_character_btver (Utilities|Casting|CastToStrangerCharacter_BTVer ControlledPawn))
  (if (>= _returnvalue_2 (Utilities|Array|Length (Variables|/Game/MallMischiefContent/Blueprints/StrangerCharacterBT/StrangerCharacter_BTVer.StrangerCharacter_BTVer_C|GetTargetLocationList _asstranger_character_btver)))
    (Class|BTFunctionLibrary|SetBlackboardValueasInt (Variables|Default|GetTargetListIndex))
    (else
      (Class|BTFunctionLibrary|SetBlackboardValueasInt (Variables|Default|GetTargetListIndex) _returnvalue_2)))
  (AI|BehaviorTree|SetBlackboardValueasVector (Variables|Default|GetCurrentTarget) (Transformation|GetActorLocation (Utilities|Array|Get(acopy) (Variables|/Game/MallMischiefContent/Blueprints/StrangerCharacterBT/StrangerCharacter_BTVer.StrangerCharacter_BTVer_C|GetTargetLocationList _asstranger_character_btver) (Class|BTFunctionLibrary|GetBlackboardValueasInt (Variables|Default|GetTargetListIndex)))))
  (AI|BehaviorTree|FinishExecute true))