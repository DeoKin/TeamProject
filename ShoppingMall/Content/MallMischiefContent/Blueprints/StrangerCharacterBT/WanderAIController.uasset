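; AI controller for wandering stranger characters, which sets up and starts their behavior tree on BeginPlay.
; It casts the controlled pawn to StrangerCharacter_BTVer, initializes WanderBlackboard, and seeds it with that character's wait time, the location of its first target actor and a zeroed integer.
; It then runs WanderBT, addressing blackboard keys by index in a key array.
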(event EventBeginPlay
  (bind _returnvalue (AI|GetBlackboard 0))
  (bind _blackboardkeys (Variables|Default|GetBlackboardKeys))
  (bind _asstranger_character_btver (Utilities|Casting|CastToStrangerCharacter_BTVer (Pawn|GetControlledPawn)))
  (Class|AIController|UseBlackboard "/Game/MallMischiefContent/Blueprints/StrangerCharacterBT/WanderBlackboard.WanderBlackboard")
  (AI|Components|Blackboard|SetValueasFloat _returnvalue (Utilities|Array|Get(acopy) _blackboardkeys) (Variables|/Game/MallMischiefContent/Blueprints/StrangerCharacterBT/StrangerCharacter_BTVer.StrangerCharacter_BTVer_C|GetWaitTime _asstranger_character_btver))
  (AI|Components|Blackboard|SetValueasVector _returnvalue (Utilities|Array|Get(acopy) _blackboardkeys 1) (Transformation|GetActorLocation (Utilities|Array|Get(acopy) (Variables|/Game/MallMischiefContent/Blueprints/StrangerCharacterBT/StrangerCharacter_BTVer.StrangerCharacter_BTVer_C|GetTargetLocationList _asstranger_character_btver))))
  (Class|BlackboardComponent|SetValueasInt _returnvalue (Utilities|Array|Get(acopy) _blackboardkeys 2))
  (AI|RunBehaviorTree "/Game/MallMischiefContent/Blueprints/StrangerCharacterBT/WanderBT.WanderBT"))

(fn ConstructionScript)