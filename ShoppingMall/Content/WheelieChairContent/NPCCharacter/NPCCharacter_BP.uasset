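; NPC character that hands its per-instance settings to an AI behavior tree for moving among a list of targets.
; On BeginPlay it initializes the blackboard, copies in list behaviour, wait time, starting target and player-notice flag, then runs the tree.
; The starting target is random for At Random and the first list entry for every other behaviour.
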(event EventBeginPlay
  (Class|AIController|UseBlackboard (AI|GetAIController self) "/Game/WheelieChairContent/NPCCharacter/AI/NPCAI_Blackboard.NPCAI_Blackboard")
  (CallFunction|TransferDatatoBlackboard)
  (AI|RunBehaviorTree (AI|GetAIController self) "/Game/WheelieChairContent/NPCCharacter/AI/NPCAI_BehaviourTree.NPCAI_BehaviourTree"))

(fn ConstructionScript)

(fn DetermineStartingIndex
  (switch Utilities|FlowControl|Switch|SwitchonTargetListBehaviour (Variables|Default|GetBehaviour)
    (:NewEnumerator3
      _)
    (:NewEnumerator0
      (return (Math|Random|RandomInteger (Utilities|Array|Length (Variables|Default|GetTargetList)))))
    (:NewEnumerator1
      _)
    (:NewEnumerator2
      _)
    (:NewEnumerator4
      _))
  (return 0))

(fn TransferDatatoBlackboard
  (bind _returnvalue (Utilities|Name|MakeLiteralName "TargetListIndex"))
  (bind _self self)
  (bind _returnvalue_2 (AI|GetAIController _self))
  (bind _returnvalue_3 (AI|GetBlackboard _returnvalue_2))
  (AI|Components|Blackboard|SetValueasEnum _returnvalue_3 (Utilities|Name|MakeLiteralName "ListBehaviour") (Variables|Default|GetBehaviour))
  (AI|Components|Blackboard|SetValueasFloat _returnvalue_3 (Utilities|Name|MakeLiteralName "WaitTime") (Variables|Default|GetWaitTime))
  (Class|BlackboardComponent|SetValueasInt _returnvalue_3 _returnvalue (CallFunction|DetermineStartingIndex))
  (AI|Components|Blackboard|SetValueasObject _returnvalue_3 (Utilities|Name|MakeLiteralName "CurrentTarget") (Utilities|Array|Get(acopy) (Variables|Default|GetTargetList) (Class|BlackboardComponent|GetValueasInt _returnvalue_3 _returnvalue)))
  (AI|Components|Blackboard|SetValueasBool _returnvalue_3 (Utilities|Name|MakeLiteralName "CanNoticePlayer") (Variables|Default|GetShouldNoticePlayer)))