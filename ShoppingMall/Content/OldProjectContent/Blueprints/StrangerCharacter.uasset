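; StrangerCharacter is an NPC character that wanders along a looping patrol route of target actors.
; On BeginPlay it optionally waits, then calls WanderToPoint to AI-move to the current entry in TargetLocationList.
; Each successful arrival advances the index, wrapping to zero at the end, then waits WaitTime before calling WanderToPoint again.
; Only the success result is handled, so a failed move stops the patrol.
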(event Custom|WanderToPoint
  ;[1 1 1] The Patrol Behaviour
  (AI|AIMoveTo self "0, 0, 0" (Utilities|Array|Get(acopy) (Variables|Default|GetTargetLocationList) (Variables|Default|GetTargetLocationIndex)) 5.0 false
    (:OnSuccess
      (if (>= (Variables|Default|GetTargetLocationIndex) (- (Utilities|Array|Length (Variables|Default|GetTargetLocationList)) 1))
        (Variables|Default|SetTargetLocationIndex 0)
        (else
          (Math|Integer|IncrementInt (Variables|Default|GetTargetLocationIndex)
            (:%20%20
              _))))
      (Utilities|FlowControl|Delay (Variables|Default|GetWaitTime))
      (CallFunction|WandertoPoint))))

(event EventBeginPlay
  ;[1 1 1] Start the wander
  (if (Variables|Default|GetStartWaiting)
    (Utilities|FlowControl|Delay (Variables|Default|GetWaitTime)))
  (CallFunction|WandertoPoint))

(fn ConstructionScript)